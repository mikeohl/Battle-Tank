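; Mortar Blueprint that sets up a mortar emplacement using tank turret, barrel and aiming components.
; On BeginPlay it initializes the TankAiming component with its turret and barrel.
; It then casts its widget component's user widget to HealthBar_BP and sets that widget's Tank reference to itself.
; The graph holds only this setup, with no tick, overlap or firing logic.
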(event EventBeginPlay
  ;[1 1 1] CommentInitialize Mortar
  (Class|TankAimingComponent|InitializeAimingComponent (Variables|Default|GetTankAiming) (Variables|Default|GetTankTurret) (Variables|Default|GetTankBarrel))
  (CallFunction|InitializeHealthBar))

(event Collision|EventActorBeginOverlap
  (params (OtherActor :type Actor%20Object%20Reference)))

(event EventTick
  (params (DeltaSeconds :type Float%20%28single-precision%29)))

(fn ConstructionScript)

(fn InitializeHealthBar
  (bind _ashealth_bar_bp (Utilities|Casting|CastToHealthBar_BP (UserInterface|GetUserWidgetObject (Variables|Default|GetWidget))))
  (Variables|/Game/UI/HealthBar_BP.HealthBar_BP_C|SetTank _ashealth_bar_bp self))